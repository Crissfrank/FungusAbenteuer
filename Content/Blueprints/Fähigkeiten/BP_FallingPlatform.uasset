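; Falling platform that plays a sound and wiggles when the player character enters its box, then moves to an end location after a reaction delay.
; A Wiggle timeline feeds into a MovePlatform timeline, which lerps the mesh outward at a duration-based rate and reverses it at quarter speed.
; The construction script applies mesh, scale and rotation to platform and end-position reference, placing the latter at the end location.
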(event `self.ReceiveBeginPlay`
  (set `self.StartLocation` (`SceneComponent.RelativeLocation` (`self.MainPlatform`))))

(event `self.Box.OnComponentBeginOverlap`
  (params (OverlappedComponent :type "PrimitiveComponent Object Reference") (OtherActor :type "Actor Object Reference") (OtherComp :type "PrimitiveComponent Object Reference") (OtherBodyIndex :type Integer) (bFromSweep :type Boolean) (SweepResult :type "HitResult Structure (by ref)"))
  (cast `/Game/ThirdPerson/Blueprints/BP_ThirdPersonCharacter` OtherActor)
  (`GameplayStatics.PlaySoundAtLocation` (`self.SoundToPlay`) (`SceneComponent.K2_GetComponentLocation` (`self.MainPlatform`)) (struct) 1.0 1.0 0.0 null null null null)
  (bind (_direction _alpha) (`Timeline|Wiggle` :!via `PlayFromStart`)
    (:`Update`
      (`SceneComponent.K2_SetRelativeLocation` (`self.MainPlatform`) (`KismetMathLibrary.VLerp` (0.0 0.0 0.0) (0.0 0.0 5.0) _alpha) false false))
    (:`Finished`
      (`KismetSystemLibrary.Delay` (`self.Reaction Time`))
      (`TimelineComponent.SetPlayRate` (`self.Move Platform`) (/ 1.0 (`self.Duration in Seconds`)))
      (bind (_direction_2 _move_track) (`Timeline|Move Platform` :!label _label)
        (:`Update`
          (`SceneComponent.K2_SetRelativeLocation` (`self.MainPlatform`) (`KismetMathLibrary.VLerp` (`self.StartLocation`) (`self.EndLocation`) _move_track) false false))
        (:`Finished`
          (if (`|EnumEquality` _direction_2 "Forward")
            (`TimelineComponent.SetPlayRate` (`self.Move Platform`) (/ 0.25 (`self.Duration in Seconds`)))
            (goto _label :!via `Reverse`)))))))

(event `self.Box.OnComponentEndOverlap`
  (params (OverlappedComponent :type "PrimitiveComponent Object Reference") (OtherActor :type "Actor Object Reference") (OtherComp :type "PrimitiveComponent Object Reference") (OtherBodyIndex :type Integer))
  (cast `/Game/ThirdPerson/Blueprints/BP_ThirdPersonCharacter` OtherActor)
  (`KismetSystemLibrary.Delay` (`self.Reaction Time`)))

(fn `UserConstructionScript`
  (bind _mainplatform (`self.MainPlatform`))
  (bind _end_platform_reference (`self.End Platform Reference`))
  (bind _platformmesh (`self.PlatformMesh`))
  (`StaticMeshComponent.SetStaticMesh` _mainplatform _platformmesh)
  (`StaticMeshComponent.SetStaticMesh` _end_platform_reference _platformmesh)
  (`SceneComponent.SetRelativeScale3D` _mainplatform (`self.Scale`))
  (`SceneComponent.SetRelativeScale3D` _end_platform_reference (`self.Scale`))
  (`SceneComponent.K2_SetRelativeRotation` _mainplatform (`self.Rotation`) false false)
  (`SceneComponent.K2_SetRelativeRotation` _end_platform_reference (`self.Rotation`) false false)
  (`SceneComponent.K2_SetRelativeLocation` _end_platform_reference (`self.EndLocation`) false false))