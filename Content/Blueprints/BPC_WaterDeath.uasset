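; BPC_WaterDeath is a component that makes its owning actor, presumably water, deadly to the player character.
; On BeginPlay it binds to the owner's begin-overlap event, checks for an exact BP_ThirdPersonCharacter class match, then calls Kill on all actors of that class, not just the overlapping one.
; An identical hit handler exists, but its binding is disconnected.
; Both handlers print True/False debug strings.
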(event `OnActorHit`
  (params (SelfActor :type "Actor Object Reference") (OtherActor :type "Actor Object Reference") (NormalImpulse :type "Vector Structure") (Hit :type "HitResult Structure (by ref)"))
  (if (== (`GameplayStatics.GetObjectClass` OtherActor) "/Game/ThirdPerson/Blueprints/BP_ThirdPersonCharacter.BP_ThirdPersonCharacter_C")
    (`KismetSystemLibrary.PrintString` "True")
    (bind _outactors (`GameplayStatics.GetAllActorsOfClass` "/Game/ThirdPerson/Blueprints/BP_ThirdPersonCharacter.BP_ThirdPersonCharacter_C"))
    (`/Game/ThirdPerson/Blueprints/BP_ThirdPersonCharacter.Kill` _outactors)
    (else
      (`KismetSystemLibrary.PrintString` "False"))))

(event `self.ReceiveBeginPlay`
  (add `Actor.OnActorBeginOverlap` (`self.GetOwner`) (delegate `Overlap`)))

(event `Overlap`
  (params (OverlappedActor :type "Actor Object Reference") (OtherActor :type "Actor Object Reference"))
  (if (== (`GameplayStatics.GetObjectClass` OtherActor) "/Game/ThirdPerson/Blueprints/BP_ThirdPersonCharacter.BP_ThirdPersonCharacter_C")
    (`KismetSystemLibrary.PrintString` "True")
    (bind _outactors (`GameplayStatics.GetAllActorsOfClass` "/Game/ThirdPerson/Blueprints/BP_ThirdPersonCharacter.BP_ThirdPersonCharacter_C"))
    (`/Game/ThirdPerson/Blueprints/BP_ThirdPersonCharacter.Kill` _outactors)
    (else
      (`KismetSystemLibrary.PrintString` "False"))))