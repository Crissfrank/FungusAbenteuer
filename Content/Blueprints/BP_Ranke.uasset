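; BP_Ranke is a spline-based actor that builds a chain of deformed meshes along its spline, likely a vine or tendril.
; The construction script divides the spline length by MeshLenght and adds a Z-forward spline mesh component for each segment.
; Tangents are clamped to the segment length, and MeshLenght is printed for debugging.
; Alternative per-point and scale-based variants are left unconnected, and the event graph is empty.
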(fn `UserConstructionScript`
  (bind _spline (`self.Spline`))
  (bind _spline_2 (`self.Spline`))
  (`KismetSystemLibrary.PrintString` (`KismetStringLibrary.Conv_DoubleToString` (`self.MeshLenght`)))
  (for _index (range (+ (`KismetMathLibrary.FTrunc` (/ (`SplineComponent.GetSplineLength` (`self.Spline`)) (`self.MeshLenght`))) 1))
    (bind _returnvalue (`AddComponent|NODE_AddSplineMeshComponent-2`))
    (`SplineMeshComponent.SetForwardAxis` _returnvalue "Z" true)
    (bind _returnvalue_2 (* _index (`self.MeshLenght`)))
    (bind _returnvalue_3 (* (+ _index 1) (`self.MeshLenght`)))
    (`SplineMeshComponent.SetStartAndEnd` _returnvalue (`SplineComponent.GetLocationAtDistanceAlongSpline` _spline_2 _returnvalue_2 "Local") (`KismetMathLibrary.ClampVectorSize` (`SplineComponent.GetTangentAtDistanceAlongSpline` _spline_2 _returnvalue_2 "Local") 0.0 (`self.MeshLenght`)) (`SplineComponent.GetLocationAtDistanceAlongSpline` _spline _returnvalue_3 "Local") (`KismetMathLibrary.ClampVectorSize` (`SplineComponent.GetTangentAtDistanceAlongSpline` _spline _returnvalue_3 "Local") 0.0 (`self.MeshLenght`)) true)))